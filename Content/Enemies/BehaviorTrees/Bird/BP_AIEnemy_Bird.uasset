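; Flying bird enemy AI character that can be shot down and switches between patrol and sprint flight speeds.
; Sphere hits from Cat-tagged actors call EnemyDeath, while Projectile-tagged bullets subtract their damage component's value from Health and are destroyed.
; Bullet hits spawn hit particles, or death particles before destroying the bird once Health runs out.
; ChangeMoveSpeed sets MaxFlySpeed based on EnemyFound.
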(event `self.ReceiveBeginPlay`
  (`SkeletalMeshComponent.Play` (`self.Mesh`) false)
  (`parent.ReceiveBeginPlay`))

(event `self.Sphere.OnComponentHit`
  (params (HitComponent :type "PrimitiveComponent Object Reference") (OtherActor :type "Actor Object Reference") (OtherComp :type "PrimitiveComponent Object Reference") (NormalImpulse :type "Vector Structure") (Hit :type "HitResult Structure (by ref)"))
  (bind _returnvalue (`SceneComponent.K2_GetComponentToWorld` HitComponent))
  (if (`KismetArrayLibrary.Array_Contains` (`Actor.Tags` OtherActor) "Cat")
    (`self.EnemyDeath`)
    (elif (`KismetArrayLibrary.Array_Contains` (`Actor.Tags` OtherActor) "Projectile")
      (bind _asbp_bullet (cast `/Game/Projectiles/BP_Bullet` OtherActor))
      (bind _output_get (set `self.Health` (- (`self.Health`) (`/Game/Components/BPC_Bullet_Damage.Damage` (`/Game/Projectiles/BP_Bullet.BPC_Bullet_Damage` _asbp_bullet)))))
      (`self.K2_DestroyActor` OtherActor)
      (if (<= _output_get 0.0)
        (`|SpawnActorFromClass` "/Game/Particles/DeathParticles_Blueprint.DeathParticles_Blueprint_C" _returnvalue "Undefined" "MultiplyWithRoot" null null)
        (`self.K2_DestroyActor`)
        (else
          (`|SpawnActorFromClass` "/Game/Particles/HitParticles.HitParticles_C" _returnvalue "Undefined" "MultiplyWithRoot" null null))))))

(fn `ChangeMoveSpeed`
  (bind _charactermovement (`self.CharacterMovement`))
  (if (`self.EnemyFound`)
    (set `CharacterMovementComponent.MaxFlySpeed` (`self.SprintSpeed`) _charactermovement)
    (else
      (set `CharacterMovementComponent.MaxFlySpeed` (`self.PatrolSpeed`) _charactermovement))))

(fn `UserConstructionScript`
  (`parent.UserConstructionScript`))