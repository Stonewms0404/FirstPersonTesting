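; Base AI enemy character that sets its health, attack and speed stats from its EnemyType (Squirrel, Duck, Cat or Bird) on BeginPlay.
; PawnSensing sight and hearing store the first-person player as the target and switch walk speed from patrol to sprint, with no reset afterwards.
; Overlapping tagged projectiles subtract their damage and destroy the enemy at zero health.
; SetPatrolPoints returns a random patrol point, while ShootProjectile is an empty stub.
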(event `self.ReceiveActorBeginOverlap`
  (params (OtherActor :type "Actor Object Reference"))
  (if (`KismetArrayLibrary.Array_Contains` (`Actor.Tags` OtherActor) "Projectile")
    (bind _asbp_projectile_base (cast `/Game/Projectiles/BP_Projectile_Base` OtherActor))
    (bind _output_get (set `self.Health` (- (`self.Health`) (`/Game/Components/BPC_ProjectileDamage.Damage` (`/Game/Projectiles/BP_Projectile_Base.BPC_ProjectileDamage` _asbp_projectile_base)))))
    (`self.K2_DestroyActor` OtherActor)
    (if (<= _output_get 0.0)
      (`self.K2_DestroyActor`))))

(event `self.ReceiveBeginPlay`
  (set `self.EnemyFound` false)
  (switch `/Game/Enemies/BaseBlueprints/EnemyType` (`self.EnemyType`)
    (:`NewEnumerator0`
      (set `self.MaxHealth` 50.0)
      (set `self.Attack` 5.0)
      (set `self.SprintSpeed` 800.0)
      (set `self.PatrolSpeed` 500.0)
      (set `self.ShootSpeed` 0.0))
    (:`NewEnumerator1`
      (set `self.MaxHealth` 200.0)
      (set `self.Attack` 25.0)
      (set `self.SprintSpeed` 500.0)
      (set `self.PatrolSpeed` 200.0))
    (:`NewEnumerator2`
      (set `self.MaxHealth` 120.0)
      (set `self.Attack` 12.0)
      (set `self.SprintSpeed` 1000.0)
      (set `self.PatrolSpeed` 300.0))
    (:`NewEnumerator3`
      (set `self.MaxHealth` 60.0)
      (set `self.Attack` 10.0)
      (set `self.SprintSpeed` 700.0)
      (set `self.PatrolSpeed` 400.0)
      (set `self.FlyingHeight` 200.0)
      (set `self.ShootSpeed` 0.0)))
  (set `self.Health` (`self.MaxHealth`)))

(event `self.PawnSensing.OnSeePawn`
  (params (Pawn :type "Pawn Object Reference"))
  (bind _asbp_first_person_character (cast `/Game/FirstPersonAssets/FirstPerson/Blueprints/BP_FirstPersonCharacter` Pawn)
    (:`then`
      (set `self.EnemyReference` _asbp_first_person_character)
      (set `self.EnemyFound` true)
      (`self.ChangeMoveSpeed`))
    (:`CastFailed`
      (if (not (`self.EnemyFound`))
        (`self.ChangeMoveSpeed`)))))

(event `self.PawnSensing.OnHearNoise`
  (params (Instigator :type "Pawn Object Reference") (Location :type "Vector Structure (by ref)") (Volume :type "Float (single-precision)"))
  (bind _asbp_first_person_character (cast `/Game/FirstPersonAssets/FirstPerson/Blueprints/BP_FirstPersonCharacter` Instigator)
    (:`then`
      (set `self.EnemyReference` _asbp_first_person_character)
      (set `self.EnemyFound` true)
      (`self.ChangeMoveSpeed`))
    (:`CastFailed`
      (if (not (`self.EnemyFound`))
        (`self.ChangeMoveSpeed`)))))

(fn `ChangeMoveSpeed`
  (bind _charactermovement (`self.CharacterMovement`))
  (if (`self.EnemyFound`)
    (set `CharacterMovementComponent.MaxWalkSpeed` (`self.SprintSpeed`) _charactermovement)
    (else
      (set `CharacterMovementComponent.MaxWalkSpeed` (`self.PatrolSpeed`) _charactermovement))))

(fn `EnemyDeath`
  (`self.K2_DestroyActor`))

(fn `SetPatrolPoints`
  (returns (PatrolPoint :type "Vector Structure"))
  (return (`KismetArrayLibrary.Array_Random` (`self.PatrolPoints`))))

(fn `ShootProjectile`)

(fn `UserConstructionScript`)