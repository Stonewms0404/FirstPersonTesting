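; Base enemy Blueprint that senses the player by sight or sound and is meant to chase them.
; PawnSensing's see and hear events pass a cast, then latch PlayerFound and set PlayerPos to None, so no target is visibly stored.
; While PlayerFound is true, Tick calls AIMoveTo toward PlayerPos every frame, using AttackRadius as acceptance radius.
; Nothing here clears the flag or performs an attack.
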(event `self.ReceiveTick`
  (params (DeltaSeconds :type "Float (single-precision)"))
  ;[0 0 0] Path towards the player if it is found
  (if (`self.PlayerFound`)
    (`|AIMoveTo` self (0.0 0.0 0.0) (`.PlayerPos` (`self.PlayerPos`)) (`self.AttackRadius`))))

(event `self.PawnSensing.OnSeePawn`
  (params (Pawn :type "Pawn Object Reference"))
  ;[0 0 0] Sensing the player
  (bind _asbp_first_person_character (cast `` Pawn))
  (set `self.PlayerFound` true)
  (set `self.PlayerPos` null _asbp_first_person_character))

(event `self.PawnSensing.OnHearNoise`
  (params (Instigator :type "Pawn Object Reference") (Location :type "Vector Structure (by ref)") (Volume :type "Float (single-precision)"))
  ;[0 0 0] Sensing the player
  (bind _asbp_first_person_character (cast `` Instigator))
  (set `self.PlayerFound` true)
  (set `self.PlayerPos` null _asbp_first_person_character))

(fn `UserConstructionScript`)