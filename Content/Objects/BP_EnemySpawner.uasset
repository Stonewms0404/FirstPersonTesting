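; Enemy spawner actor that periodically spawns a random AI enemy at its own transform.
; On BeginPlay it picks a random interval once and starts a looping timer at that fixed rate.
; Each tick of the timer calls SpawnEnemy, which chooses Duck, Squirrel or Bird with equal odds.
; Spawns ignore collisions, and the Blueprint sets no limit on how many enemies accumulate.
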(event `self.ReceiveBeginPlay`
  (bind _output_get (set `self.SpawnTimer` (`KismetMathLibrary.RandomFloatInRange` 5.0 10.0)))
  (`KismetSystemLibrary.K2_SetTimerDelegate` (delegate `EV_SpawnEnemy`) _output_get true))

(event `EV_SpawnEnemy`
  (`self.SpawnEnemy`))

(fn `SpawnEnemy`
  (bind _returnvalue (`self.GetTransform`))
  (bind _output_get (set `self.RandomEnemy` (`KismetMathLibrary.RandomInteger` 3)))
  (switch `int` _output_get
    (:`0`
      (`|SpawnActorFromClass` "/Game/Enemies/BehaviorTrees/Duck/BP_AIEnemy_Duck.BP_AIEnemy_Duck_C" _returnvalue "AlwaysSpawn" "MultiplyWithRoot" null null))
    (:`1`
      (`|SpawnActorFromClass` "/Game/Enemies/BehaviorTrees/Squirrel/BP_AIEnemy_Squirrel.BP_AIEnemy_Squirrel_C" _returnvalue "AlwaysSpawn" "MultiplyWithRoot" null null))
    (:`2`
      (`|SpawnActorFromClass` "/Game/Enemies/BehaviorTrees/Bird/BP_AIEnemy_Bird.BP_AIEnemy_Bird_C" _returnvalue "AlwaysSpawn" "MultiplyWithRoot" null null))))

(fn `UserConstructionScript`)