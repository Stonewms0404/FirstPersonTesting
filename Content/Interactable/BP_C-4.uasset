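; C-4 explosive actor that shows an interact prompt and detonates on a timer.
; PlayerDetect overlap stores the first-person character and adds an "E to Interact" widget, then clears the reference and collapses the widget on exit.
; Detonate, which has no caller here, waits, spawns an explosion effect, rescales the DMG damage field and destroys the actor.
; BeginPlay shows the Time component and copies Damage into the bullet damage component.
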(event `Detonate`
  (`KismetSystemLibrary.Delay` 5.0)
  (`|SpawnActorFromClass` "/Game/StarterContent/Blueprints/Blueprint_Effect_Explosion.Blueprint_Effect_Explosion_C" (`self.GetTransform` self) "AlwaysSpawn" "OverrideRootScale" null null)
  (`SceneComponent.SetRelativeScale3D` (`self.DMG`) (`self.DamageFieldScale`))
  (`self.K2_DestroyActor`))

(event `self.PlayerDetect.OnComponentBeginOverlap`
  (params (OverlappedComponent :type "PrimitiveComponent Object Reference") (OtherActor :type "Actor Object Reference") (OtherComp :type "PrimitiveComponent Object Reference") (OtherBodyIndex :type Integer) (bFromSweep :type Boolean) (SweepResult :type "HitResult Structure (by ref)"))
  (bind _asbp_first_person_character (cast `/Game/FirstPersonAssets/FirstPerson/Blueprints/BP_FirstPersonCharacter` OtherActor))
  (set `self.PlayerRef` _asbp_first_person_character)
  (bind _returnvalue (`|CreateWidget` "/Game/UserInterface/WB_E_to_Interact.WB_E_to_Interact_C"))
  (`UserWidget.AddToViewport` _returnvalue 0))

(event `self.PlayerDetect.OnComponentEndOverlap`
  (params (OverlappedComponent :type "PrimitiveComponent Object Reference") (OtherActor :type "Actor Object Reference") (OtherComp :type "PrimitiveComponent Object Reference") (OtherBodyIndex :type Integer))
  (cast `/Game/FirstPersonAssets/FirstPerson/Blueprints/BP_FirstPersonCharacter` OtherActor)
  (set `self.PlayerRef` null)
  (`Widget.SetVisibility` (stale `self.PlayerDetect.OnComponentBeginOverlap` _returnvalue) "Collapsed"))

(event `self.ReceiveBeginPlay`
  (`SceneComponent.SetVisibility` (`self.Time`) true false)
  (set `/Game/Components/BPC_Bullet_Damage.Damage` (`KismetMathLibrary.FTrunc` (`self.Damage`)) (`self.BPC_Bullet_Damage`)))

(fn `UserConstructionScript`)