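; BP_Cat_Projectile is a projectile that turns into a cat AI enemy when it expires or hits something.
; BeginPlay applies speed to ProjectileMovement and damage to BPCBulletDamage, then starts a despawn timer.
; Hits push physics-simulating components and destroy the projectile at once; other hits trigger a very short despawn timer.
; Both endings share logic that spawns an explosion effect and BP_AIEnemy_Cat with its behavior tree.
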(event `self.ReceiveBeginPlay`
  (bind _projectilemovement (`self.ProjectileMovement`))
  ;[0 0 0] When the bullet is spawned the speed and damage are set
  (bind _output_get (set `ProjectileMovementComponent.InitialSpeed` (`self.Projectile Speed`) _projectilemovement))
  (set `ProjectileMovementComponent.MaxSpeed` _output_get _projectilemovement)
  (set `/Game/Components/BPC_Bullet_Damage.Damage` (`self.Projectile Damage`) (`self.BPC_Bullet_Damage`))
  (`KismetSystemLibrary.K2_SetTimerDelegate` (delegate `DespawnTimer`) 5.0))

(event `DespawnTimer`
  (bind _returnvalue (`self.K2_GetActorLocation`))
  ;[0 0 0] When the bullet is spawned the speed and damage are set
  (`self.K2_DestroyActor`)
  ;[0 0 0] When the bullet hits an object and if that object is simulating physics, add impulse to that object and destroy the bullet
  (`|SpawnActorFromClass` "/Game/StarterContent/Blueprints/Blueprint_Effect_Explosion.Blueprint_Effect_Explosion_C" (`KismetMathLibrary.Conv_VectorToTransform` _returnvalue) "AdjustIfPossibleButAlwaysSpawn" "MultiplyWithRoot" null null :!label _label)
  (`AIBlueprintHelperLibrary.SpawnAIFromClass` "/Game/Enemies/BehaviorTrees/Cat/BP_AIEnemy_Cat.BP_AIEnemy_Cat_C" "/Game/Enemies/BehaviorTrees/Cat/BT_AIEnemy_Cat.BT_AIEnemy_Cat" _returnvalue (struct) false null))

(event `self.ReceiveHit`
  (params (MyComp :type "PrimitiveComponent Object Reference") (Other :type "Actor Object Reference") (OtherComp :type "PrimitiveComponent Object Reference") (bSelfMoved :type Boolean) (HitLocation :type "Vector Structure") (HitNormal :type "Vector Structure") (NormalImpulse :type "Vector Structure") (Hit :type "HitResult Structure (by ref)"))
  ;[0 0 0] When the bullet hits an object and if that object is simulating physics, add impulse to that object and destroy the bullet
  (if (`SceneComponent.IsSimulatingPhysics` OtherComp "None")
    (`PrimitiveComponent.AddImpulseAtLocation` OtherComp (`self.GetVelocity`) (`self.K2_GetActorLocation`) "None")
    (`self.K2_DestroyActor`)
    (goto _label)
    (else
      (`KismetSystemLibrary.K2_SetTimerDelegate` (delegate `DespawnTimer`) 0.05))))

(fn `UserConstructionScript`)