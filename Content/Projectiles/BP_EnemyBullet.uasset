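; Enemy bullet projectile that pushes physics objects it hits; no damage is applied in these graphs.
; On BeginPlay it sets its ProjectileMovement initial and max speed from a base speed and multiplier, then starts a lifetime despawn timer.
; On Hit, a physics-simulating component receives an impulse scaled from the bullet's velocity and the bullet is destroyed at once.
; Any other hit schedules the despawn after a very short delay.
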(event `self.ReceiveBeginPlay`
  (bind _projectilemovement (`self.ProjectileMovement`))
  ;[0 0 0] When the bullet is spawned the speed and damage are set
  (bind _output_get (set `ProjectileMovementComponent.InitialSpeed` (* (`self.Projectile Speed`) (`self.Speed Mult`)) _projectilemovement))
  (set `ProjectileMovementComponent.MaxSpeed` _output_get _projectilemovement)
  (`KismetSystemLibrary.K2_SetTimerDelegate` (delegate `DespawnTimer`) 5.0))

(event `DespawnTimer`
  ;[0 0 0] When the bullet is spawned the speed and damage are set
  (`self.K2_DestroyActor`))

(event `self.ReceiveHit`
  (params (MyComp :type "PrimitiveComponent Object Reference") (Other :type "Actor Object Reference") (OtherComp :type "PrimitiveComponent Object Reference") (bSelfMoved :type Boolean) (HitLocation :type "Vector Structure") (HitNormal :type "Vector Structure") (NormalImpulse :type "Vector Structure") (Hit :type "HitResult Structure (by ref)"))
  ;[0 0 0] When the bullet hits an object and if that object is simulating physics, add impulse to that object and destroy the bullet
  (if (`SceneComponent.IsSimulatingPhysics` OtherComp "None")
    (`PrimitiveComponent.AddImpulseAtLocation` OtherComp (* (`self.GetVelocity`) 100.0) (`self.K2_GetActorLocation`) "None")
    (`self.K2_DestroyActor`)
    (else
      (`KismetSystemLibrary.K2_SetTimerDelegate` (delegate `DespawnTimer`) 0.05))))

(fn `UserConstructionScript`)