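; BP_Bullet is a weapon projectile that adds slight random spread to its rotation and sets its speed when spawned.
; If player 0's first-person character has a valid weapon, it sets its damage component by weapon type (D Eagle, AK or Shotgun) and starts a despawn timer.
; On hit, it pushes physics-simulating components with a velocity-based impulse and destroys itself, otherwise despawning after a brief delay.
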(event `self.ReceiveBeginPlay`
  (bind (_returnvalue_roll _returnvalue_pitch _returnvalue_yaw) (`KismetMathLibrary.BreakRotator` (`self.K2_GetActorRotation`)))
  (bind _returnvalue (`KismetMathLibrary.RandomFloatInRange` -1.0 1.0))
  (bind _projectilemovement (`self.ProjectileMovement`))
  (bind _bpc_bullet_damage (`self.BPC_Bullet_Damage`))
  ;[0 0 0] When the bullet is spawned the speed and damage are set
  (`self.K2_SetActorRotation` (`KismetMathLibrary.MakeRotator` _returnvalue_roll (+ _returnvalue_pitch _returnvalue) (+ _returnvalue_yaw _returnvalue)))
  (bind _output_get (set `ProjectileMovementComponent.InitialSpeed` (* (`self.Projectile Speed`) (`self.Speed Mult`)) _projectilemovement))
  (set `ProjectileMovementComponent.MaxSpeed` _output_get _projectilemovement)
  (bind _asbp_first_person_character (cast `/Game/FirstPersonAssets/FirstPerson/Blueprints/BP_FirstPersonCharacter` (`GameplayStatics.GetPlayerCharacter` 0)))
  (`/Engine/EditorBlueprintResources/StandardMacros.IsValid` (`/Game/FirstPersonAssets/FirstPerson/Blueprints/BP_FirstPersonCharacter.CurrentWeapon` _asbp_first_person_character)
    (:`Is Valid`
      (switch `/Game/FirstPersonAssets/FirstPerson/Blueprints/WeaponTypes` "NewEnumerator0"
        (:`NewEnumerator0`
          (set `/Game/Components/BPC_Bullet_Damage.Damage` 30 _bpc_bullet_damage))
        (:`NewEnumerator1`
          (set `/Game/Components/BPC_Bullet_Damage.Damage` 10 _bpc_bullet_damage))
        (:`NewEnumerator2`
          (set `/Game/Components/BPC_Bullet_Damage.Damage` 20 _bpc_bullet_damage)))
      (`KismetSystemLibrary.K2_SetTimerDelegate` (delegate `DespawnTimer`) 5.0))))

(event `DespawnTimer`
  ;[0 0 0] When the bullet is spawned the speed and damage are set
  (`self.K2_DestroyActor`))

(event `self.ReceiveHit`
  (params (MyComp :type "PrimitiveComponent Object Reference") (Other :type "Actor Object Reference") (OtherComp :type "PrimitiveComponent Object Reference") (bSelfMoved :type Boolean) (HitLocation :type "Vector Structure") (HitNormal :type "Vector Structure") (NormalImpulse :type "Vector Structure") (Hit :type "HitResult Structure (by ref)"))
  ;[0 0 0] When the bullet hits an object and if that object is simulating physics, add impulse to that object and destroy the bullet
  (if (`SceneComponent.IsSimulatingPhysics` OtherComp "None")
    (`PrimitiveComponent.AddImpulseAtLocation` OtherComp (* (`self.GetVelocity`) 100.0) (`self.K2_GetActorLocation`) "None")
    (`self.K2_DestroyActor`)
    (else
      (`KismetSystemLibrary.K2_SetTimerDelegate` (delegate `DespawnTimer`) 0.05))))

(fn `UserConstructionScript`)