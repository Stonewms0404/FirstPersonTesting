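; BP_Activation is a trigger actor that activates tagged platforms when a first-person character holding a key enters its box.
; On BeginPlay it caches every BP_Base_Platform in the level.
; The box overlap checks the character's HasKey flag, then, through a DoOnce, calls EvActivate on each cached platform whose actor tag matches its Tag variable, so activation fires only once.
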(event `self.ReceiveBeginPlay`
  (bind _outactors (`GameplayStatics.GetAllActorsOfClass` "/Game/Matt-Learning/BP_Base_Platform.BP_Base_Platform_C"))
  (set `self.PlatformList` _outactors))

(event `self.Box.OnComponentBeginOverlap`
  (params (OverlappedComponent :type "PrimitiveComponent Object Reference") (OtherActor :type "Actor Object Reference") (OtherComp :type "PrimitiveComponent Object Reference") (OtherBodyIndex :type Integer) (bFromSweep :type Boolean) (SweepResult :type "HitResult Structure (by ref)"))
  (bind _asbp_first_person_character (cast `/Game/FirstPersonAssets/FirstPerson/Blueprints/BP_FirstPersonCharacter` OtherActor))
  (if (`/Game/FirstPersonAssets/FirstPerson/Blueprints/BP_FirstPersonCharacter.bHasKey` _asbp_first_person_character)
    (`/Engine/EditorBlueprintResources/StandardMacros.DoOnce` false
      (:`Completed`
        (for _array_element (`self.PlatformList`)
          (if (`self.ActorHasTag` _array_element (`self.Tag`))
            (`/Game/Matt-Learning/BP_Base_Platform.evActivate` _array_element)))))))

(fn `UserConstructionScript`)