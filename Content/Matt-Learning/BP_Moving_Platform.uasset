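; BP_Moving_Platform is a platform actor that shuttles its Cube back and forth between its starting position and EndLocation.
; On BeginPlay it stores the Cube's relative location, sets the timeline play rate and begins moving after StartDelay.
; The TM_Movement timeline lerps the position, then pauses for StopDelay at each end before playing or reversing.
; Older manual-alpha and VInterpTo movement logic remains unconnected.
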(event `self.ReceiveBeginPlay`
  (set `self.StartingLocation` (`SceneComponent.RelativeLocation` (`self.Cube`)))
  (`TimelineComponent.SetPlayRate` (`self.TM_Movement`) (`self.New Rate`))
  (`KismetSystemLibrary.Delay` (`self.Start Delay`))
  (`self.Go Forward`))

(event `Go Forward`
  (bind _stop_delay (`self.Stop Delay`))
  (bind (_direction _alpha) (`Timeline|TM_Movement` :!label _label)
    (:`Update`
      (`SceneComponent.K2_SetRelativeLocation` (`self.Cube`) (`KismetMathLibrary.VLerp` (`self.StartingLocation`) (`self.EndLocation`) _alpha) false false))
    (:`Finished`
      (if (`|EnumEquality` _direction "Forward")
        (`KismetSystemLibrary.Delay` _stop_delay)
        (`self.Go Back`)
        (else
          (`KismetSystemLibrary.Delay` _stop_delay)
          (`self.Go Forward`))))))

(event `Go Back`
  (goto _label :!via `Reverse`))

(event `self.ReceiveTick`
  (params (DeltaSeconds :type "Float (single-precision)")))

(fn `UserConstructionScript`)