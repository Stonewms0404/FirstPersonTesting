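; Moving platform Blueprint that, once EvActivate fires, slides its Cube back and forth between its starting relative location and EndLocation.
; Tick drives the motion, lerping by a fixed per-frame Alpha step, so speed depends on frame rate, and flipping direction at each end.
; An alternative timeline ping-pong with stop delays, gated by PlayerOn, is present but nothing starts it, and the Box overlap events are empty.
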(event `self.ReceiveBeginPlay`
  (set `self.StartingLocation` (`SceneComponent.RelativeLocation` (`self.Cube`)))
  (`TimelineComponent.SetPlayRate` (`self.TM_Movement`) (`self.New Rate`)))

(event `Go Forward`
  (bind _stop_delay (`self.Stop Delay`))
  (if (`self.PlayerOn`)
    (bind (_direction _alpha) (`Timeline|TM_Movement` :!label _label)
      (:`Update`
        (`SceneComponent.K2_SetRelativeLocation` (`self.Cube`) (`KismetMathLibrary.VLerp` (`self.StartingLocation`) (`self.EndLocation`) _alpha) false false))
      (:`Finished`
        (if (`|EnumEquality` _direction "Forward")
          (`KismetSystemLibrary.Delay` _stop_delay)
          (`self.Go Back`)
          (else
            (`KismetSystemLibrary.Delay` _stop_delay)
            (`self.Go Forward`)))))))

(event `Stop`
  (goto _label :!via `Stop`))

(event `Go Back`
  (if (`self.PlayerOn`)
    (goto _label :!via `Reverse`)))

(event `self.ReceiveTick`
  (params (DeltaSeconds :type "Float (single-precision)"))
  (if (`self.Active`)
    (if (`self.Forward`)
      (`SceneComponent.K2_SetRelativeLocation` (`self.Cube`) (`KismetMathLibrary.VLerp` (`self.StartingLocation`) (`self.EndLocation`) (`self.Alpha`)) false false)
      (bind _output_get (set `self.Alpha` (`KismetMathLibrary.FClamp` (+ (`self.Alpha`) 0.01))))
      (if (== _output_get 1.0)
        (set `self.Forward` false)
        (set `self.Alpha` 0.0))
      (else
        (`SceneComponent.K2_SetRelativeLocation` (`self.Cube`) (`KismetMathLibrary.VLerp` (`self.EndLocation`) (`self.StartingLocation`) (`self.Alpha`)) false false)
        (bind _output_get_2 (set `self.Alpha` (`KismetMathLibrary.FClamp` (+ (`self.Alpha`) 0.01))))
        (if (== _output_get_2 1.0)
          (set `self.Forward` true)
          (set `self.Alpha` 0.0))))))

(event `self.Box.OnComponentBeginOverlap`
  (params (OverlappedComponent :type "PrimitiveComponent Object Reference") (OtherActor :type "Actor Object Reference") (OtherComp :type "PrimitiveComponent Object Reference") (OtherBodyIndex :type Integer) (bFromSweep :type Boolean) (SweepResult :type "HitResult Structure (by ref)")))

(event `self.Box.OnComponentEndOverlap`
  (params (OverlappedComponent :type "PrimitiveComponent Object Reference") (OtherActor :type "Actor Object Reference") (OtherComp :type "PrimitiveComponent Object Reference") (OtherBodyIndex :type Integer)))

(event `self.evActivate`
  (set `self.Active` true))

(fn `UserConstructionScript`)